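; Elevator actor that moves from its starting position along a timeline-driven offset.
; BeginPlay waits a short random delay, then stores the actor's location as the start position.
; Tick polls the ElevatorStart flag, clears it and plays the MyCounter timeline, whose updates add MyNewZPosition to the stored position without sweeping.
; Nothing in this Blueprint sets ElevatorStart to true.
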(event `self.ReceiveBeginPlay`
  (`KismetSystemLibrary.Delay` (`KismetMathLibrary.RandomFloatInRange` 0.0 2.0))
  (set `self.myStartPosition` (`self.K2_GetActorLocation`)))

(event `self.ReceiveTick`
  (params (DeltaSeconds :type "Float (single-precision)"))
  (if (`self.elevatorStart`)
    (set `self.elevatorStart` false)
    (bind (_direction _mynewzposition) (`Timeline|myCounter`)
      (:`Update`
        (`self.K2_SetActorLocation` (+ _mynewzposition (`self.myStartPosition`)))))))

(fn `UserConstructionScript`)