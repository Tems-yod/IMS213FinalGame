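; bp_button is a one-shot pressure-plate button that starts the elevator and shows a cinematic camera view.
; The first overlap by any actor sets a trigger flag, snaps the button to a hardcoded position and plays a click.
; It blends player 0's view to the found CineCameraActor and sets ElevatorStart on the found Bp_elevator.
; After a short delay it destroys the CineCameraActor, with no explicit view-target reset.
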(event `self.ReceiveActorBeginOverlap`
  (params (OtherActor :type "Actor Object Reference"))
  (if (not (`self.buttonTriggered`))
    (set `self.buttonTriggered` true)
    (`self.K2_SetActorLocation` (200.0 400.0 1356.78))
    (`GameplayStatics.PlaySoundAtLocation` "/Game/MyAssets/420975__hefler__pressure-plate-click.420975__hefler__pressure-plate-click" (`self.K2_GetActorLocation`) (struct) 1.0 1.0 0.0 null null null null)
    (bind _returnvalue (`GameplayStatics.GetActorOfClass` "/Script/CinematicCamera.CineCameraActor"))
    (`PlayerController.SetViewTargetWithBlend` (`PlayerState.GetPlayerController` (`GameplayStatics.GetPlayerState` 0)) _returnvalue 1.0 "VTBlend_Linear" 0.0 false)
    (bind _returnvalue_2 (`GameplayStatics.GetActorOfClass` "/Game/MyBlueprints/bp_elevator.bp_elevator_C"))
    (bind _asbp_elevator (cast `/Game/MyBlueprints/bp_elevator` _returnvalue_2))
    (set `/Game/MyBlueprints/bp_elevator.elevatorStart` true _asbp_elevator)
    (`KismetSystemLibrary.Delay` 5.0)
    (bind _returnvalue_3 (`GameplayStatics.GetActorOfClass` "/Script/CinematicCamera.CineCameraActor"))
    (`self.K2_DestroyActor` _returnvalue_3)))

(fn `UserConstructionScript`)